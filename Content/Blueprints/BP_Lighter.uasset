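; BP_Lighter is an actor that blinks red, yellow and green lights in an endless sequence.
; The construction script gathers the three lights into an array.
; From BeginPlay, a self-looping Delay toggles the current light's visibility on a fixed interval, counting down twice the Blooms value so each blink is an on-off pair.
; When the count runs out, it moves to the next light, wrapping back to the first.
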(event `self.ReceiveBeginPlay`
  (set `self.PrivateBlooms` (* (`self.Blooms`) 2))
  (`KismetSystemLibrary.Delay` 0.75 :!label _label)
  (`SceneComponent.ToggleVisibility` (`|GetArrayItem` (`self.AllLights`) (`self.CurrColor`)) false)
  (bind _result (`/Engine/EditorBlueprintResources/StandardMacros.DecrementInt` (`self.PrivateBlooms`))
    (:`  `
      (if (!= _result 0)
        (goto _label)
        (else
          (set `self.PrivateBlooms` (* (`self.Blooms`) 2))
          (bind _result_2 (`/Engine/EditorBlueprintResources/StandardMacros.IncrementInt` (`self.CurrColor`))
            (:`  `
              (if (< _result_2 (`KismetArrayLibrary.Array_Length` (`self.AllLights`)))
                (goto _label)
                (else
                  (set `self.CurrColor` 0)
                  (goto _label))))))))))

(fn `UserConstructionScript`
  (bind _alllights (`self.AllLights`))
  (`KismetArrayLibrary.Array_Add` _alllights (`self.Red`))
  (`KismetArrayLibrary.Array_Add` _alllights (`self.Yellow`))
  (`KismetArrayLibrary.Array_Add` _alllights (`self.Green`)))