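; Bonus ball for the ping game that moves in the XY plane and bounces off whatever blocks it.
; BeginPlay picks a random velocity heading toward negative X with random sideways drift.
; While IsGame is set by StartGame, Tick sweeps the Sphere by that velocity times Speed, reflecting it off hit normals; PauseGame halts movement.
; When IsUsedTime is on, a Time countdown destroys the ball on expiry, even while paused.
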(event `self.ReceiveBeginPlay`
  (set `self.BallDirections` (`KismetMathLibrary.MakeVector` (`KismetMathLibrary.RandomFloatInRange` -400.0 -800.0) (`KismetMathLibrary.RandomFloatInRange` -400.0 400.0))))

(event `self.ReceiveTick`
  (params (DeltaSeconds :type "Float (single-precision)"))
  (if (`self.IsUsedTime`)
    (bind _output_get (set `self.Time` (- (`self.Time`) DeltaSeconds)))
    (if (< _output_get 0.0)
      (`self.K2_DestroyActor`)
      (else
        (if (`self.IsGame`) :!label _label
          (bind _sweephitresult (`SceneComponent.K2_AddLocalOffset` (`self.Sphere`) (* (* (`self.BallDirections`) (`self.Speed`)) DeltaSeconds) true false))
          (bind (_bblockinghit _binitialoverlap _time _distance _location _impactpoint _normal) (`GameplayStatics.BreakHitResult` _sweephitresult))
          (if _bblockinghit
            (bind (_returnvalue_x _returnvalue_y) (`KismetMathLibrary.BreakVector` (`KismetMathLibrary.GetReflectionVector` (`self.BallDirections`) _normal)))
            (set `self.BallDirections` (`KismetMathLibrary.MakeVector` _returnvalue_x _returnvalue_y))))))
    (else
      (goto _label))))

(fn `PauseGame`
  (set `self.IsGame` false))

(fn `StartGame`
  (set `self.IsGame` true))

(fn `UserConstructionScript`)