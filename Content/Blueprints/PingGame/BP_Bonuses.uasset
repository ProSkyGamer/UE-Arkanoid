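; BP_Bonuses is a moving pickup in the ping game that grants one of three random bonuses.
; BeginPlay picks the type and colors the sphere green, red or yellow, and Tick moves it with a swept offset.
; OnHit, gated by IsGame, sets player speed, makes the ball super or spawns a bonus ball, then destroys the pickup.
; The Hit event is empty, leaving an older cast-based copy of that logic disconnected.
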(event `self.ReceiveBeginPlay`
  (set `self.BonusType` (`KismetMathLibrary.RandomIntegerInRange` 0 2))
  (`SceneComponent.K2_AddLocalOffset` (`self.Sphere`) (`self.BonusOffset`) false false)
  (if (== (`self.BonusType`) 0)
    (`PrimitiveComponent.SetMaterial` (`self.Sphere`) 0 "/Game/Blueprints/PingGame/CubeMaterials/Green.Green")
    (elif (== (`self.BonusType`) 1)
      (`PrimitiveComponent.SetMaterial` (`self.Sphere`) 0 "/Game/Blueprints/PingGame/CubeMaterials/Red.Red")
      (elif (== (`self.BonusType`) 2)
        (`PrimitiveComponent.SetMaterial` (`self.Sphere`) 0 "/Game/Blueprints/PingGame/CubeMaterials/Yellow.Yellow")
        (else
          (`self.K2_DestroyActor`))))))

(event `self.ReceiveTick`
  (params (DeltaSeconds :type "Float (single-precision)"))
  (`SceneComponent.K2_AddLocalOffset` (`self.Sphere`) (* DeltaSeconds (* (`self.Direction`) (`self.Speed`))) true false))

(event `self.ReceiveHit`
  (params (MyComp :type "PrimitiveComponent Object Reference") (Other :type "Actor Object Reference") (OtherComp :type "PrimitiveComponent Object Reference") (bSelfMoved :type Boolean) (HitLocation :type "Vector Structure") (HitNormal :type "Vector Structure") (NormalImpulse :type "Vector Structure") (Hit :type "HitResult Structure (by ref)")))

(fn `OnHit`
  (bind _ball (`self.Ball`))
  (if (`self.IsGame`)
    (if (== (`self.BonusType`) 0)
      (bind _outactors (`GameplayStatics.GetAllActorsOfClass` "/Game/Blueprints/PingGame/BP_Player.BP_Player_C"))
      (for _array_element _outactors
        (set `/Game/Blueprints/PingGame/BP_Player.PlayerSpeed` 75 _array_element))
      (elif (== (`self.BonusType`) 1)
        (set `/Game/Blueprints/PingGame/BP_Ball.IsSuper` true _ball)
        (`PrimitiveComponent.SetMaterial` (`/Game/Blueprints/PingGame/BP_Ball.Sphere` _ball) 0 "/Game/Blueprints/PingGame/CubeMaterials/Red.Red")
        (else
          (`|SpawnActorFromClass` "/Game/Blueprints/PingGame/BP_BonusBall.BP_BonusBall_C" (`KismetMathLibrary.Conv_VectorToTransform` (+ (`SceneComponent.K2_GetComponentLocation` (`self.Sphere`)) (`self.BallOffset`))) "Undefined" "OverrideRootScale" null null))))
    (`self.K2_DestroyActor`)))

(fn `UserConstructionScript`)