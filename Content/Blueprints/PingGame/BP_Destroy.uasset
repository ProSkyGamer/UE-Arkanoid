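; BP_Destroy is the kill zone and end-of-game handler for a ping-style ball game.
; When a BP_Ball overlaps its Box, it destroys the ball, ends the game on all players, shows the loss UI and clears IsGame on all bonuses.
; Overlapping bonuses are simply destroyed.
; A separate WinGame function shows the win UI, ends the game on players and destroys all balls.
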(event `self.Box.OnComponentBeginOverlap`
  (params (OverlappedComponent :type "PrimitiveComponent Object Reference") (OtherActor :type "Actor Object Reference") (OtherComp :type "PrimitiveComponent Object Reference") (OtherBodyIndex :type Integer) (bFromSweep :type Boolean) (SweepResult :type "HitResult Structure (by ref)"))
  (bind _asbp_ball (cast `/Game/Blueprints/PingGame/BP_Ball` OtherActor)
    (:`then`
      (`self.K2_DestroyActor` _asbp_ball)
      (bind _outactors (`GameplayStatics.GetAllActorsOfClass` "/Game/Blueprints/PingGame/BP_Player.BP_Player_C"))
      (for _array_element _outactors
        (`/Game/Blueprints/PingGame/BP_Player.EndGame` _array_element))
      (`/Game/Blueprints/PingGame/BP_Interface.LoseGame` (`self.UI`))
      (bind _outactors_2 (`GameplayStatics.GetAllActorsOfClass` "/Game/Blueprints/PingGame/BP_Bonuses.BP_Bonuses_C"))
      (for _array_element_2 _outactors_2
        (set `/Game/Blueprints/PingGame/BP_Bonuses.IsGame` false _array_element_2)))
    (:`CastFailed`
      (bind _asbp_bonuses (cast `/Game/Blueprints/PingGame/BP_Bonuses` OtherActor))
      (`self.K2_DestroyActor` _asbp_bonuses))))

(fn `UserConstructionScript`)

(fn `WinGame`
  (`/Game/Blueprints/PingGame/BP_Interface.WinGame` (`self.UI`))
  (bind _outactors (`GameplayStatics.GetAllActorsOfClass` "/Game/Blueprints/PingGame/BP_Player.BP_Player_C"))
  (for _array_element _outactors
    (`/Game/Blueprints/PingGame/BP_Player.EndGame` _array_element))
  (bind _outactors_2 (`GameplayStatics.GetAllActorsOfClass` "/Game/Blueprints/PingGame/BP_Ball.BP_Ball_C"))
  (for _array_element_2 _outactors_2
    (`self.K2_DestroyActor` _array_element_2)))