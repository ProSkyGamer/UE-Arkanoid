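; BP_Player is the player-controlled piece in PingGame, sliding its Cube along local X while a game flag is set by StartGame and cleared by EndGame.
; Tick merges the AD axis with a second axis key input, so agreeing inputs do not stack speed and opposing ones cancel.
; Movement is a swept per-frame offset not scaled by delta time.
; Hits on BP_Bonuses actors call their OnHit.
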(event `self.ReceiveTick`
  (params (DeltaSeconds :type "Float (single-precision)"))
  (bind _returnvalue (`self.GetInputAxisValue`))
  (if (`self.IsGame`)
    (if (!= (`self.GetInputAxisKeyValue`) 0.0)
      (if (!= _returnvalue 0.0)
        (if (> _returnvalue 0.0)
          (if (> (`self.GetInputAxisKeyValue`) 0.0)
            (`SceneComponent.K2_AddLocalOffset` (`self.Cube`) (`KismetMathLibrary.MakeVector` (* (`self.PlayerSpeed`) (`self.GetInputAxisValue`))) true false))
          (elif (< (`self.GetInputAxisKeyValue`) 0.0)
            (`SceneComponent.K2_AddLocalOffset` (`self.Cube`) (`KismetMathLibrary.MakeVector` (* (`self.PlayerSpeed`) (`self.GetInputAxisValue`))) true false)))
        (elif (> (`self.GetInputAxisKeyValue`) 0.0)
          (`SceneComponent.K2_AddLocalOffset` (`self.Cube`) (`KismetMathLibrary.MakeVector` (* 1.0 (`self.PlayerSpeed`))) true false)
          (else
            (`SceneComponent.K2_AddLocalOffset` (`self.Cube`) (`KismetMathLibrary.MakeVector` (* -1.0 (`self.PlayerSpeed`))) true false))))
      (elif (!= (`self.GetInputAxisValue`) 0.0)
        (`SceneComponent.K2_AddLocalOffset` (`self.Cube`) (`KismetMathLibrary.MakeVector` (* (`self.GetInputAxisValue`) (`self.PlayerSpeed`))) true false)))))

(event `self.ReceiveHit`
  (params (MyComp :type "PrimitiveComponent Object Reference") (Other :type "Actor Object Reference") (OtherComp :type "PrimitiveComponent Object Reference") (bSelfMoved :type Boolean) (HitLocation :type "Vector Structure") (HitNormal :type "Vector Structure") (NormalImpulse :type "Vector Structure") (Hit :type "HitResult Structure (by ref)"))
  (bind _asbp_bonuses (cast `/Game/Blueprints/PingGame/BP_Bonuses` Other))
  (`/Game/Blueprints/PingGame/BP_Bonuses.OnHit` _asbp_bonuses))

(fn `EndGame`
  (set `self.IsGame` false))

(fn `StartGame`
  (set `self.IsGame` true))

(fn `UserConstructionScript`)